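; Title-screen game mode that builds the title menu UI and starts the game.
; On BeginPlay it caches the GI_Main game instance (quitting if the cast fails), shows the mouse cursor and displays the title widget.
; Loading screen and option widgets are reused from the game instance, or created and stored there, then added hidden.
; GameStart reveals the loading screen, requests a stream load of Lv_Main001, then opens that level.
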(event `self.ReceiveBeginPlay`
  (bind _wbp_option (`/Game/00_sakane/BluePrint/GameInstance/GI_Main.WBP_Option` (`self.GI_Main`)))
  (bind _wbp_loadingscreen (`/Game/00_sakane/BluePrint/GameInstance/GI_Main.WBP_LoadingScreen` (`self.GI_Main`)))
  (`|ExecutionSequence`
    (:`then_0`
      (bind _asgi_main (cast `/Game/00_sakane/BluePrint/GameInstance/GI_Main` (`GameplayStatics.GetGameInstance`))
        (:`then`
          (set `self.GI_Main` _asgi_main)
          (set `PlayerController.bShowMouseCursor` true (`GameplayStatics.GetPlayerController` 0)))
        (:`CastFailed`
          (`KismetSystemLibrary.QuitGame` null "Quit"))))
    (:`then_1`
      (bind _returnvalue (`|CreateWidget` "/Game/00_sakane/BluePrint/UI/WBP_Title.WBP_Title_C"))
      (bind _output_get (set `self.WBP_Title` _returnvalue))
      (`UserWidget.AddToViewport` _output_get 0))
    (:`then_2`
      (`/Engine/EditorBlueprintResources/StandardMacros.IsValid` _wbp_loadingscreen
        (:`Is Valid`
          (set `self.WBP_LoadingScreen` _wbp_loadingscreen))
        (:`Is Not Valid`
          (bind _returnvalue_2 (`|CreateWidget` "/Game/00_sakane/BluePrint/UI/WBP_LoadingScreen.WBP_LoadingScreen_C"))
          (bind _output_get_2 (set `/Game/00_sakane/BluePrint/GameInstance/GI_Main.WBP_LoadingScreen` _returnvalue_2 (`self.GI_Main`)))
          (set `self.WBP_LoadingScreen` _output_get_2)))
      (`UserWidget.AddToViewport` (`self.WBP_LoadingScreen`) 0)
      (`Widget.SetVisibility` (`self.WBP_LoadingScreen`) "Hidden"))
    (:`then_3`
      (`/Engine/EditorBlueprintResources/StandardMacros.IsValid` _wbp_option
        (:`Is Valid`
          (set `self.WBP_Option` _wbp_option))
        (:`Is Not Valid`
          (bind _returnvalue_3 (`|CreateWidget` "/Game/00_sakane/BluePrint/UI/WBP_Option.WBP_Option_C"))
          (bind _output_get_3 (set `/Game/00_sakane/BluePrint/GameInstance/GI_Main.WBP_Option` _returnvalue_3 (`self.GI_Main`)))
          (set `self.WBP_Option` _output_get_3)))
      (`UserWidget.AddToViewport` (`self.WBP_Option`) 0)
      (`Widget.SetVisibility` (`self.WBP_Option`) "Hidden"))))

(event `/Game/00_sakane/BluePrint/GameMode/Interface/BPI_GM_Title.GameStart`
  (`Widget.SetVisibility` (`self.WBP_LoadingScreen`) "Visible")
  (`GameplayStatics.LoadStreamLevelBySoftObjectPtr` "/Game/00_sakane/Level/Lv_Main001.Lv_Main001" true)
  (`GameplayStatics.OpenLevelBySoftObjectPtr` "/Game/00_sakane/Level/Lv_Main001.Lv_Main001"))

(fn `UserConstructionScript`)