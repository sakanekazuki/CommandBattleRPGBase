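; Battle GameMode that runs a turn-based fight between spawned player and enemy BP_BattleCharacters, with help from CPPBattleSubSystem.
; Toggles action, skill and target widgets to collect each player's choice, though targeting and execution only use the first character.
; CharacterDead removes the fallen, then starts the next turn or opens Lv_Main001 once either side is wiped out.
; Action ordering and NextAction are empty stubs, and Run only prints.
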(event `self.ReceiveBeginPlay`
  ;[1 1 1] ゲームインスタンス取得
  (bind _asgi_main (cast `/Game/00_sakane/BluePrint/GameInstance/GI_Main` (`GameplayStatics.GetGameInstance`))
    (:`then`
      (set `self.GI_Main` _asgi_main)
      (`|ExecutionSequence`
        (:`then_0`
          (bind _returnvalue (`|CreateWidget` "/Game/00_sakane/BluePrint/UI/WBP_SkillSelect.WBP_SkillSelect_C"))
          (bind _output_get (set `self.wbp_skillSelect` _returnvalue))
          (`UserWidget.AddToViewport` _output_get 0)
          (`Widget.SetVisibility` (`self.wbp_skillSelect`) "Hidden"))
        (:`then_1`
          (bind _returnvalue_2 (`|CreateWidget` "/Game/00_sakane/BluePrint/UI/WBP_ActionSelect.WBP_ActionSelect_C"))
          (bind _output_get_2 (set `self.wbp_actionSelect` _returnvalue_2))
          (`UserWidget.AddToViewport` _output_get_2 0)
          (`Widget.SetVisibility` (`self.wbp_actionSelect`) "Hidden"))
        (:`then_2`
          (bind _returnvalue_3 (`|CreateWidget` "/Game/00_sakane/BluePrint/UI/WBP_TargetSelect.WBP_TargetSelect_C"))
          (bind _output_get_3 (set `self.wbp_TargetSelect` _returnvalue_3))
          (`UserWidget.AddToViewport` _output_get_3 0)
          (`Widget.SetVisibility` (`self.wbp_TargetSelect`) "Hidden"))
        (:`then_3`
          (`CPP_BattleSubSystem.BattleStart` (subsystem `CPP_BattleSubSystem`))
          (`self.BattleStart`)
          (`self.ActionSelectStart`))))
    (:`CastFailed`
      (`KismetSystemLibrary.PrintString` "エラーが発生したためタイトルに戻ります")
      (`GameplayStatics.LoadStreamLevelBySoftObjectPtr` "/Game/00_sakane/Level/Lv_Title.Lv_Title" true)
      (`GameplayStatics.OpenLevelBySoftObjectPtr` "/Game/00_sakane/Level/Lv_Title.Lv_Title"))))

(event `/Game/00_sakane/BluePrint/GameMode/Interface/BPI_GM_Battle.ActionSelectStart`
  (`Widget.SetVisibility` (`self.wbp_actionSelect`) "Visible")
  (`Widget.SetVisibility` (`self.wbp_skillSelect`) "Hidden")
  (`Widget.SetVisibility` (`self.wbp_TargetSelect`) "Hidden"))

(event `/Game/00_sakane/BluePrint/GameMode/Interface/BPI_GM_Battle.SkillSelect`
  (params (Skill :type Integer))
  (`Widget.SetVisibility` (`self.wbp_TargetSelect`) "Visible")
  (`Widget.SetVisibility` (`self.wbp_skillSelect`) "Hidden")
  (`Widget.SetVisibility` (`self.wbp_actionSelect`) "Hidden"))

(event `/Game/00_sakane/BluePrint/GameMode/Interface/BPI_GM_Battle.TargetSelect`
  (params (Target :type Integer))
  (`/Game/00_sakane/BluePrint/Player/BP_BattleCharacter.SetAttackTarget` (`|GetArrayItem` (`self.playerBattleCharacters`)) (`|GetArrayItem` (`self.enemyBattleCharacters`) Target))
  (`/Engine/EditorBlueprintResources/StandardMacros.IncrementInt` (`self.selectCharacterValue`)
    (:`  `
      (if (== (`KismetArrayLibrary.Array_Length` (`self.playerBattleCharacters`)) (`self.selectCharacterValue`))
        (`self.Set Action Order`)
        (`self.SkillExecution`)
        (else
          ;[1 1 1] 次のキャラクターのスキルを選択
          (`/Game/00_sakane/BluePrint/GameMode/Interface/BPI_GM_Battle.ActionSelect` "NewEnumerator0"))))))

(event `/Game/00_sakane/BluePrint/GameMode/Interface/BPI_GM_Battle.ActionSelect`
  (params (Action :type "/Game/00_sakane/BluePrint/Enum/E_ActionType Enum" :default "NewEnumerator0"))
  (switch `/Game/00_sakane/BluePrint/Enum/E_ActionType` Action
    (:`NewEnumerator0`
      (`Widget.SetVisibility` (`self.wbp_skillSelect`) "Visible")
      (`Widget.SetVisibility` (`self.wbp_TargetSelect`) "Hidden")
      (`Widget.SetVisibility` (`self.wbp_actionSelect`) "Hidden"))
    (:`NewEnumerator1`
      (`KismetSystemLibrary.PrintString` "逃げる"))))

(event `/Game/00_sakane/BluePrint/GameMode/Interface/BPI_GM_Battle.CharacterDead`
  (params (DeadCharacter :type "Actor Object Reference"))
  (bind _asbp_battle_character (cast `/Game/00_sakane/BluePrint/Player/BP_BattleCharacter` DeadCharacter)
    (:`then`
      (if (`self.ActorHasTag` DeadCharacter "Player")
        (bind _returnvalue (`KismetArrayLibrary.Array_RemoveItem` (`self.playerBattleCharacters`) _asbp_battle_character))
        (if _returnvalue
          (`KismetSystemLibrary.PrintString` "取り除きに成功")
          (if (<= (`KismetArrayLibrary.Array_Length` (`self.playerBattleCharacters`)) 0)
            (`KismetSystemLibrary.PrintString` "プレイヤーの負け")
            (`GameplayStatics.LoadStreamLevelBySoftObjectPtr` "/Game/00_sakane/Level/Lv_Main001.Lv_Main001" true :!label _label)
            (`GameplayStatics.OpenLevelBySoftObjectPtr` "/Game/00_sakane/Level/Lv_Main001.Lv_Main001")
            (else
              (`self.NextTurn`)))
          (else
            (`KismetSystemLibrary.PrintString` "取り除きに失敗")))
        (else
          (bind _returnvalue_2 (`KismetArrayLibrary.Array_RemoveItem` (`self.enemyBattleCharacters`) _asbp_battle_character))
          (if _returnvalue_2
            (`KismetSystemLibrary.PrintString` "取り除きに成功")
            (if (<= (`KismetArrayLibrary.Array_Length` (`self.enemyBattleCharacters`)) 0)
              (`KismetSystemLibrary.PrintString` "プレイヤーの勝利")
              (goto _label)
              (else
                (`self.NextTurn`)))
            (else
              (`KismetSystemLibrary.PrintString` "取り除きに失敗"))))))
    (:`CastFailed`
      (`KismetSystemLibrary.PrintString` "変換に失敗"))))

(fn `BattleStart`
  (bind _array (`|MakeArray` 0 0 0))
  (bind _output (`|GetArrayItem` (`self.enemyBattleCharacters`) (`KismetArrayLibrary.Array_LastIndex` (`self.enemyBattleCharacters`))))
  (bind _output_2 (`|GetArrayItem` (`self.playerBattleCharacters`) (`KismetArrayLibrary.Array_LastIndex` (`self.playerBattleCharacters`))))
  (bind _tags (`Actor.Tags` _output))
  (bind _tags_2 (`Actor.Tags` _output_2))
  (`|ExecutionSequence`
    (:`then_0`
      ;[1 1 1] プレイヤー側のキャラクター生成
      (for _array_element (`self.playerPositions`)
        (bind _returnvalue (`|SpawnActorFromClass` "/Game/00_sakane/BluePrint/Player/BP_BattleCharacter.BP_BattleCharacter_C" (`KismetMathLibrary.MakeTransform` _array_element (struct :`Yaw` 90.0)) "Undefined" "MultiplyWithRoot" null "/Game/00_sakane/BluePrint/DataAsset/PlayerParty/DA_Hero.DA_Hero" null))
        (`KismetArrayLibrary.Array_Add` (`self.playerBattleCharacters`) _returnvalue)
        (`KismetArrayLibrary.Array_Add` _tags_2 "Player")
        (set `Actor.Tags` _tags_2 _output_2)))
    (:`then_1`
      ;[1 1 1] 敵キャラクター生成
      (for (_ _array_index) _array
        (bind _returnvalue_2 (`|SpawnActorFromClass` "/Game/00_sakane/BluePrint/Player/BP_BattleCharacter.BP_BattleCharacter_C" (`KismetMathLibrary.MakeTransform` (`|GetArrayItem` (`CPP_BattleSubSystem.PositionCalculation` (subsystem `CPP_BattleSubSystem`) (`KismetArrayLibrary.Array_Length` _array) 250.0) _array_index) (struct :`Yaw` 270.0)) "Undefined" "MultiplyWithRoot" null "/Game/00_sakane/BluePrint/DataAsset/PlayerParty/DA_Hero.DA_Hero" null))
        (`KismetArrayLibrary.Array_Add` (`self.enemyBattleCharacters`) _returnvalue_2)
        (`KismetArrayLibrary.Array_Add` _tags "Enemy")
        (set `Actor.Tags` _tags _output)))))

(fn `NextAction`)

(fn `NextTurn`
  ;[1 1 1] ターンを進める
  (`CPP_BattleSubSystem.NextTurn` (subsystem `CPP_BattleSubSystem`))
  ;[1 1 1] スキル選択状態にする
  (set `self.turnState` "NewEnumerator2")
  ;[1 1 1] 戦闘UI表示・フォーカス
  (`/Game/00_sakane/BluePrint/GameMode/Interface/BPI_GM_Battle.ActionSelectStart`)
  ;[1 1 1] スキルを選択したキャラクター数を戻す
  (set `self.selectCharacterValue` 0))

(fn `Set Action Order`)

(fn `SkillExecution`
  (`/Game/00_sakane/BluePrint/Player/BP_BattleCharacter.SkillExecution` (`|GetArrayItem` (`self.playerBattleCharacters`)))
  (`KismetSystemLibrary.PrintString` "攻撃した"))

(fn `UserConstructionScript`)