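; GM_Main01 is the main game mode, handling screen widget setup, the transition into battle and the options menu.
; On BeginPlay it reuses or creates loading and option widgets cached on GI_Main, adds them hidden and hides the cursor, returning to Lv_Title if the cast fails.
; BattleStart updates FieldState, shows loading and opens Lv_Battle.
; Menu and MenuClose toggle the option widget and mouse cursor.
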(event `self.ReceiveBeginPlay`
  (bind _asgi_main (cast `/Game/00_sakane/BluePrint/GameInstance/GI_Main` (`GameplayStatics.GetGameInstance`))
    (:`then`
      (bind _output_get (set `self.GI_Main` _asgi_main))
      ;[1 1 1] ロード画面取得＆非表示（生成されていない場合生成）
      (`/Engine/EditorBlueprintResources/StandardMacros.IsValid` (`/Game/00_sakane/BluePrint/GameInstance/GI_Main.WBP_LoadingScreen` _output_get)
        (:`Is Valid`
          (set `self.wbp_LoadingScreen` (`/Game/00_sakane/BluePrint/GameInstance/GI_Main.WBP_LoadingScreen` (`self.GI_Main`))))
        (:`Is Not Valid`
          (bind _returnvalue (`|CreateWidget` "/Game/00_sakane/BluePrint/UI/WBP_LoadingScreen.WBP_LoadingScreen_C"))
          (bind _output_get_2 (set `/Game/00_sakane/BluePrint/GameInstance/GI_Main.WBP_LoadingScreen` _returnvalue (`self.GI_Main`)))
          (set `self.wbp_LoadingScreen` _output_get_2)))
      (`UserWidget.AddToViewport` (`self.wbp_LoadingScreen`) 0)
      (`Widget.SetVisibility` (`self.wbp_LoadingScreen`) "Hidden")
      ;[1 1 1] オプション画面取得＆非表示（生成されていない場合生成）
      (`/Engine/EditorBlueprintResources/StandardMacros.IsValid` (`/Game/00_sakane/BluePrint/GameInstance/GI_Main.WBP_Option` (`self.GI_Main`))
        (:`Is Valid`
          (set `self.wbp_Option` (`/Game/00_sakane/BluePrint/GameInstance/GI_Main.WBP_Option` (`self.GI_Main`))))
        (:`Is Not Valid`
          (bind _returnvalue_2 (`|CreateWidget` "/Game/00_sakane/BluePrint/UI/WBP_Option.WBP_Option_C"))
          (bind _output_get_3 (set `/Game/00_sakane/BluePrint/GameInstance/GI_Main.WBP_Option` _returnvalue_2 (`self.GI_Main`)))
          (set `self.wbp_Option` _output_get_3)))
      (`UserWidget.AddToViewport` (`self.wbp_Option`) 0)
      (`Widget.SetVisibility` (`self.wbp_Option`) "Hidden")
      ;[1 1 1] マウスカーソル非表示
      (set `PlayerController.bShowMouseCursor` false (`GameplayStatics.GetPlayerController` 0)))
    (:`CastFailed`
      ;[1 1 1] ゲームインスタンスのキャストに失敗した場合、タイトル画面に戻す
      (`KismetSystemLibrary.PrintString` "エラーが発生したためタイトルに戻ります")
      (`GameplayStatics.LoadStreamLevelBySoftObjectPtr` "/Game/00_sakane/Level/Lv_Title.Lv_Title" true)
      (`GameplayStatics.OpenLevelBySoftObjectPtr` "/Game/00_sakane/Level/Lv_Title.Lv_Title"))))

(event `/Game/00_sakane/BluePrint/GameMode/Interface/BPI_GM_Main01.BattleStart`
  ;[1 1 1] 戦闘開始
  (set `self.fieldState` "NewEnumerator1")
  (`Widget.SetVisibility` (`self.wbp_LoadingScreen`) "Visible")
  (`GameplayStatics.LoadStreamLevelBySoftObjectPtr` "/Game/00_sakane/Level/Lv_Battle.Lv_Battle" true)
  (`GameplayStatics.OpenLevelBySoftObjectPtr` "/Game/00_sakane/Level/Lv_Battle.Lv_Battle"))

(event `/Game/00_sakane/BluePrint/GameMode/Interface/BPI_GM_Main01.Menu`
  ;[1 1 1] メニュー表示
  (`Widget.SetVisibility` (`self.wbp_Option`) "Visible")
  (set `PlayerController.bShowMouseCursor` true (`GameplayStatics.GetPlayerController` 0)))

(event `/Game/00_sakane/BluePrint/GameMode/Interface/BPI_GM_Main01.MenuClose`
  ;[1 1 1] メニュー非表示
  (`Widget.SetVisibility` (`self.wbp_Option`) "Hidden")
  (set `PlayerController.bShowMouseCursor` false (`GameplayStatics.GetPlayerController` 0)))

(fn `UserConstructionScript`)