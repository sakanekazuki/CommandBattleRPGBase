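; BP_BattleCharacter is a battle character that takes its skeletal mesh and animation class from a DaCharacter data reference on BeginPlay.
; SetAttackTarget accumulates actors in a target array, and SkillExecution applies a fixed damage amount to each of them; the array is never cleared here.
; Any damage received, regardless of amount, prints a defeat message, reports the death to the GameMode and destroys the actor.
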(event `self.ReceiveBeginPlay`
  ;[1 1 1] メッシュ、アニメーション設定
  (`SkeletalMeshComponent.SetSkeletalMeshAsset` (`self.SkeletalMesh`) (`/Game/00_sakane/BluePrint/DataAsset/DA_BattleCharacter.skeletaleMesh` (`self.da_Character`)))
  (`SkeletalMeshComponent.SetAnimInstanceClass` (`self.SkeletalMesh`) (`/Game/00_sakane/BluePrint/DataAsset/DA_BattleCharacter.animationInstance` (`self.da_Character`))))

(event `self.ReceiveAnyDamage`
  (params (Damage :type "Float (single-precision)") (DamageType :type "DamageType Object Reference") (InstigatedBy :type "Controller Object Reference") (DamageCauser :type "Actor Object Reference"))
  (`KismetSystemLibrary.PrintString` "倒れた")
  (message `/Game/00_sakane/BluePrint/GameMode/Interface/BPI_GM_Battle.CharacterDead` (`GameplayStatics.GetGameMode`) self)
  (`self.K2_DestroyActor`))

(event `self.SkillExecution`
  (for _array_element (`self.attackTargetActors`)
    (`GameplayStatics.ApplyDamage` _array_element 1.0)))

(fn `SetAttackTarget`
  (params (Target :type "Actor Object Reference"))
  (`KismetArrayLibrary.Array_Add` (`self.attackTargetActors`) Target))

(fn `UserConstructionScript`)