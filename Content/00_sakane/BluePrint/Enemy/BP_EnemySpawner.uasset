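; BP_EnemySpawner is an actor that continuously spawns BP_EnemyBase enemies within its box area.
; BeginPlay starts a looping half-second timer that calls Spawn, with no limit on count.
; Each spawn takes a random X and Y inside the Box component, scaled by the actor's scale, and keeps the actor's own Z with zero rotation.
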(event `self.ReceiveBeginPlay`
  (`KismetSystemLibrary.K2_SetTimerDelegate` (delegate `Spawn`) 0.5 true))

(event `Spawn`
  (bind _box (`self.Box`))
  (`|SpawnActorFromClass` "/Game/00_sakane/BluePrint/Enemy/BP_EnemyBase.BP_EnemyBase_C" (`KismetMathLibrary.MakeTransform` (`KismetMathLibrary.MakeVector` (.x (`KismetMathLibrary.RandomPointInBoundingBox` (`SceneComponent.K2_GetComponentLocation` _box) (* (`BoxComponent.BoxExtent` _box) (.scale (`self.GetTransform`))))) (.y (`KismetMathLibrary.RandomPointInBoundingBox` (`SceneComponent.K2_GetComponentLocation` _box) (* (`BoxComponent.BoxExtent` _box) (.scale (`self.GetTransform`))))) (.z (`self.K2_GetActorLocation`)))) "Undefined" "MultiplyWithRoot" null null))

(fn `UserConstructionScript`)